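; BP_Mule is a character that takes damage and performs a randomized montage attack.
; Damage lowers clamped HP, then either plays a hit-reaction montage or destroys the actor at zero.
; PlayAttack blocks re-entry, plays one of three random montage sections and disables movement until completion or interruption restores walking.
; The ControlSpeed timeline drives montage play rate from the AttackSpeed animation curve, so the animation shapes its own pacing.
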(event `self.ReceiveAnyDamage`
  (params (Damage :type "Float (single-precision)") (DamageType :type "DamageType Object Reference") (InstigatedBy :type "Controller Object Reference") (DamageCauser :type "Actor Object Reference"))
  (bind _output_get (set `self.CurrentHP` (`KismetMathLibrary.FClamp` (- (`self.CurrentHP`) Damage) 0.0 (`self.MaxHP`))))
  (if (<= _output_get 0.0)
    (`self.K2_DestroyActor`)
    (else
      (`|PlayMontage` (`self.Mesh`) "/Game/KYS/Mules/Anim/Animations/React/AM_HitReaction.AM_HitReaction"))))

(event `PlayAttack`
  (bind _charactermovement (`self.CharacterMovement`))
  (bind _returnvalue (`SkeletalMeshComponent.GetAnimInstance` (`self.Mesh`)))
  (if (not (`self.IsAttacking`))
    (set `self.IsAttacking` true)
    (`|PlayMontage` (`self.Mesh`) "/Game/KYS/Mules/Anim/Animations/Attak/AM_MuleAttack.AM_MuleAttack" 1.0 0.0 (`|GetArrayItem` (`self.Attacks`) (`KismetMathLibrary.RandomIntegerInRange` 0 2))
      (:`then`
        (`CharacterMovementComponent.DisableMovement` _charactermovement)
        (`Timeline|ControlSpeed` :!via `PlayFromStart`
          (:`Update`
            (`AnimInstance.Montage_SetPlayRate` _returnvalue "/Game/KYS/Mules/Anim/Animations/Attak/AM_MuleAttack.AM_MuleAttack" (`AnimInstance.GetCurveValue` _returnvalue "AttackSpeed")))))
      (:`OnCompleted`
        (set `self.IsAttacking` false :!label _label)
        (`CharacterMovementComponent.SetMovementMode` _charactermovement "MOVE_Walking" 0))
      (:`OnInterrupted`
        (goto _label)))))

(fn `UserConstructionScript`)