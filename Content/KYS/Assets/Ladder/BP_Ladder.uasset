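; BP_Ladder is a ladder actor that shows the player's Sam pawn a floating prompt inside either of its two interaction areas.
; Each area has its own TextRender and starts a fast looping timer on overlap, then clears it and hides the text on exit.
; Each tick of that timer sets Land or Climb text from Sam's IsClimbing state and turns it toward the camera.
; The graph only drives prompts and contains no climbing movement.
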(event `self.ReceiveBeginPlay`
  (bind _asbp_sam (cast `/Game/KYS/SamPorter/BP_Sam` (`GameplayStatics.GetPlayerPawn` 0)))
  (set `self.SamPorter` _asbp_sam))

(event `self.InteractionArea.OnComponentBeginOverlap`
  (params (OverlappedComponent :type "PrimitiveComponent Object Reference") (OtherActor :type "Actor Object Reference") (OtherComp :type "PrimitiveComponent Object Reference") (OtherBodyIndex :type Integer) (bFromSweep :type Boolean) (SweepResult :type "HitResult Structure (by ref)"))
  (if (== OtherActor (`self.SamPorter`))
    (bind _output_get (set `self.Text` (`self.TextRender`)))
    (bind _returnvalue (`KismetSystemLibrary.K2_SetTimerDelegate` (delegate `ShowText`) 0.05 true))
    (set `self.LookTimerHandle` _returnvalue)))

(event `self.InteractionArea.OnComponentEndOverlap`
  (params (OverlappedComponent :type "PrimitiveComponent Object Reference") (OtherActor :type "Actor Object Reference") (OtherComp :type "PrimitiveComponent Object Reference") (OtherBodyIndex :type Integer))
  (if (== OtherActor (`self.SamPorter`))
    (`KismetSystemLibrary.K2_ClearAndInvalidateTimerHandle` (`self.LookTimerHandle`))
    (`SceneComponent.SetVisibility` (`self.Text`) false false)))

(event `ShowText`
  (`self.ChoiceText` (`/Game/KYS/SamPorter/BP_Sam.IsClimbing` (`self.SamPorter`)) (stale `self.InteractionArea.OnComponentBeginOverlap` _output_get)))

(event `self.InteractionArea1.OnComponentBeginOverlap`
  (params (OverlappedComponent :type "PrimitiveComponent Object Reference") (OtherActor :type "Actor Object Reference") (OtherComp :type "PrimitiveComponent Object Reference") (OtherBodyIndex :type Integer) (bFromSweep :type Boolean) (SweepResult :type "HitResult Structure (by ref)"))
  (if (== OtherActor (`self.SamPorter`))
    (bind _output_get (set `self.Text` (`self.TextRender1`)))
    (bind _returnvalue (`KismetSystemLibrary.K2_SetTimerDelegate` (delegate `CustomEvent`) 0.05 true))
    (set `self.LookTimerHandle` _returnvalue)))

(event `self.InteractionArea1.OnComponentEndOverlap`
  (params (OverlappedComponent :type "PrimitiveComponent Object Reference") (OtherActor :type "Actor Object Reference") (OtherComp :type "PrimitiveComponent Object Reference") (OtherBodyIndex :type Integer))
  (if (== OtherActor (`self.SamPorter`))
    (`KismetSystemLibrary.K2_ClearAndInvalidateTimerHandle` (`self.LookTimerHandle`))
    (`SceneComponent.SetVisibility` (`self.Text`) false false)))

(event `CustomEvent`
  (`self.ChoiceText` (`/Game/KYS/SamPorter/BP_Sam.IsClimbing` (`self.SamPorter`)) (stale `self.InteractionArea1.OnComponentBeginOverlap` _output_get)))

(fn `ChoiceText`
  (params (IsClimbing :type Boolean) (TextIn :type "TextRenderComponent Object Reference"))
  (returns (TextOut :type "TextRenderComponent Object Reference"))
  (locals (Land :type Text :default "NSLOCTEXT(\"[91F3C2A962B57117DAE1FB3E92FA0DA6]\", \"CD4AF8F747DDE06694D5DFA4B518407D\", \"F : Land\")") (Climb :type Text :default "NSLOCTEXT(\"[91F3C2A962B57117DAE1FB3E92FA0DA6]\", \"E47426FE4E2FD784B38A82AC8BE162ED\", \"F : Climb\")"))
  (if IsClimbing
    (`TextRenderComponent.K2_SetText` TextIn (`local.Land`))
    (`SceneComponent.SetVisibility` TextIn true true)
    (`self.LookCamera` TextIn)
    (return TextIn)
    (else
      (`TextRenderComponent.K2_SetText` TextIn (`local.Climb`))
      (`SceneComponent.SetVisibility` TextIn true true)
      (`self.LookCamera` TextIn)
      (return TextIn))))

(fn `LookCamera`
  (params (Text :type "TextRenderComponent Object Reference"))
  (bind (_returnvalue_x _returnvalue_y _returnvalue_z) (`KismetMathLibrary.BreakVector` (`SceneComponent.K2_GetComponentLocation` Text)))
  (bind (_returnvalue_x_2 _returnvalue_y_2 _returnvalue_z_2) (`KismetMathLibrary.BreakVector` (`self.K2_GetActorLocation` (`GameplayStatics.GetPlayerCameraManager` 0))))
  (`SceneComponent.K2_SetWorldRotation` Text (`KismetMathLibrary.FindLookAtRotation` (`KismetMathLibrary.MakeVector` _returnvalue_x _returnvalue_y _returnvalue_z) (`KismetMathLibrary.MakeVector` _returnvalue_x_2 _returnvalue_y_2 _returnvalue_z_2)) false false))

(fn `UserConstructionScript`)