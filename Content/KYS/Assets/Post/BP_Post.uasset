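; BP_Post is an interactable actor that shows a text prompt when the player's BP_Sam pawn is nearby and destroys itself when interacted with.
; BeginPlay caches the Sam pawn, and InteractionArea overlaps by that pawn show or hide the TextRender.
; While the text is shown, a looping short-interval timer runs LookAtCamera to rotate it toward the player camera, and end overlap clears the timer.
; Interact only prints a debug string before destroying the actor.
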(event `self.ReceiveBeginPlay`
  (bind _asbp_sam (cast `/Game/KYS/SamPorter/BP_Sam` (`GameplayStatics.GetPlayerPawn` 0)))
  (set `self.SamPorter` _asbp_sam))

(event `/Game/KYS/Assets/BPI_Interactable.Interact`
  (`KismetSystemLibrary.PrintString` "get")
  (`self.K2_DestroyActor`))

(event `self.InteractionArea.OnComponentBeginOverlap`
  (params (OverlappedComponent :type "PrimitiveComponent Object Reference") (OtherActor :type "Actor Object Reference") (OtherComp :type "PrimitiveComponent Object Reference") (OtherBodyIndex :type Integer) (bFromSweep :type Boolean) (SweepResult :type "HitResult Structure (by ref)"))
  (if (== OtherActor (`self.SamPorter`))
    (if (not (`SceneComponent.IsVisible` (`self.TextRender`)))
      (`SceneComponent.SetVisibility` (`self.TextRender`) true true)
      (`self.LookAtCamera`)
      (`KismetSystemLibrary.K2_SetTimer` null "LookAtCamera" 0.05 true))))

(event `self.InteractionArea.OnComponentEndOverlap`
  (params (OverlappedComponent :type "PrimitiveComponent Object Reference") (OtherActor :type "Actor Object Reference") (OtherComp :type "PrimitiveComponent Object Reference") (OtherBodyIndex :type Integer))
  (if (== OtherActor (`self.SamPorter`))
    (`SceneComponent.SetVisibility` (`self.TextRender`) false true)
    (`KismetSystemLibrary.K2_ClearTimer` null "LookAtCamera")))

(fn `LookAtCamera`
  (bind (_returnvalue_x _returnvalue_y _returnvalue_z) (`KismetMathLibrary.BreakVector` (`SceneComponent.K2_GetComponentLocation` (`self.TextRender`))))
  (bind (_returnvalue_x_2 _returnvalue_y_2 _returnvalue_z_2) (`KismetMathLibrary.BreakVector` (`self.K2_GetActorLocation` (`GameplayStatics.GetPlayerCameraManager` 0))))
  (`SceneComponent.K2_SetWorldRotation` (`self.TextRender`) (`KismetMathLibrary.FindLookAtRotation` (`KismetMathLibrary.MakeVector` _returnvalue_x _returnvalue_y _returnvalue_z) (`KismetMathLibrary.MakeVector` _returnvalue_x_2 _returnvalue_y_2 _returnvalue_z_2)) false false))

(fn `UserConstructionScript`)